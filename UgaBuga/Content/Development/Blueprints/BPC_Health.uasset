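; Health component that tracks its owner's health and death state and broadcasts health-changed and death events.
; On BeginPlay it binds to the owner's any-damage event.
; While alive, each hit clamps current health without subtracting damage, updates the dead flag and fires the death event regardless of the result.
; The current-health RepNotify broadcasts the change and prints the owner's name and health for debugging.
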(event `self.ReceiveBeginPlay`
  (add `Actor.OnTakeAnyDamage` (`self.GetOwner`) (delegate `HandleDamage`)))

(event `HandleDamage`
  (params (DamagedActor :type "Actor Object Reference") (Damage :type "Float (single-precision)") (DamageType :type "DamageType Object Reference") (InstigatedBy :type "Controller Object Reference") (DamageCauser :type "Actor Object Reference"))
  (if (not (`self.BisDead`))
    (bind _output_get (set `self.CurrentHealth` (`KismetMathLibrary.FClamp` (`self.CurrentHealth`) 0.0 (`self.MaxHealth`))))
    (if true
      (set `self.BisDead` (<= _output_get 0.0))
      (`self.OnDeath`))))

(fn `OnRep_CurrentHealth`
  (`self.OnHealthChanged`)
  (`KismetSystemLibrary.PrintString` (`KismetStringLibrary.Concat_StrStr` (`KismetSystemLibrary.GetDisplayName` (`self.GetOwner`)) " can: " (`KismetStringLibrary.Conv_DoubleToString` (`self.CurrentHealth`))) true true (struct :`G` 0.66 :`B` 1.0 :`A` 1.0) 5.0))